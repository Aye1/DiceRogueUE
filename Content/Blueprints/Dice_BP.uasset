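; Physics-driven six-sided die actor with per-face data shown on face widgets and a color set by divinity.
; RollDice applies a random impulse at a random location, rerolling too-weak vectors, and starts a minimum-roll timer.
; Each Tick picks the up face by comparing widget altitudes (world X) and ends the roll once the timer has passed and velocity is zero.
; Dispatchers report roll start and stop, face changes and mouse hover.
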(event MouseInput|EventActorBeginCursorOver
  (Default|CallDiceMouseEnter self)
  (Utilities|String|LogString "Mouse over"))

(event Collision|EventActorBeginOverlap
  (params (OtherActor :type Actor%20Object%20Reference)))

(event EventTick
  (params (DeltaSeconds :type Float%20%28single-precision%29))
  (Roll|GetUpFacefromWorldLocation)
  (|SetIsInMotion)
  (Utilities|CheckIsRollFinished))

(event EventBeginPlay
  (Setup|InitFaceValues))

(event MouseInput|EventActorEndCursorOver
  (Default|CallDiceMouseExit self))

(fn ConstructionScript
  (Setup|CreateFaceWidgetArray))

(fn RollDice
  (Default|CallDiceStartedRolling self)
  (Utilities|String|LogString "Starting roll")
  (Variables|Default|SetIsRolling true)
  (Variables|Default|SetMinRollTimePassed false)
  (bind _result (Roll|MakeRandomVectorwithThreshold -2e+02 2e+02 5e+01))
  (Physics|AddImpulseatLocation (Variables|Default|GetCube) _result (Utilities|MakeRandomVector -5e+01 5e+01) "None")
  (Roll|StartRollTimer)
  (return))

(fn StartRollTimer
  (Utilities|Time|SetTimerbyFunctionName 0 "EndRollTimer" 1.0))

(fn EndRollTimer
  (Variables|Default|SetMinRollTimePassed true)
  (Utilities|Time|ClearandInvalidateTimerbyHandle (Variables|Default|GetMinRollTimer)))

(fn InitFaceValues
  (for (_array_element _array_index) (Variables|Default|GetFaceWidgetArray)
    (bind _asface_widget_bp (Utilities|Casting|CastToFaceWidget_BP (UserInterface|GetWidget _array_element))
      (:then
        (Default|SetFaceInfo _asface_widget_bp (Utilities|Array|Get(acopy) (Variables|Default|GetFaces) _array_index))
        (Utilities|Struct|SetmembersinFace_Structure (Utilities|Array|Get(acopy) (Variables|Default|GetFaces) _array_index) (Variables|Default|GetId)))
      (:CastFailed
        (Utilities|String|LogString "Cast failed - see Dice_Blueprint - InitFaceValues"))))
  (return))

(fn GetUpFacefromWorldLocation
  (LocalVariables|SetMaxAltitude -1e+05)
  (LocalVariables|SetMaxAltitudeFace -1)
  (for (_array_element _array_index) (Variables|Default|GetFaceWidgetArray)
    (if (> (Utilities|GetWorldAltitude _array_element) (LocalVariables|GetMaxAltitude))
      (LocalVariables|SetMaxAltitude (Utilities|GetWorldAltitude _array_element))
      (LocalVariables|SetMaxAltitudeFace (+ _array_index 1))))
  (if (!= (Variables|Default|GetFaceUp) (LocalVariables|GetMaxAltitudeFace))
    (Variables|Default|SetFaceUp (LocalVariables|GetMaxAltitudeFace))
    (Variables|Default|SetFaceUpInfo (Utilities|Array|Get(acopy) (Variables|Default|GetFaces) (- (LocalVariables|GetMaxAltitudeFace) 1)))
    (Default|CallDiceFaceUpChanged (Utilities|Array|Get(acopy) (Variables|Default|GetFaces) (- (LocalVariables|GetMaxAltitudeFace) 1))))
  (return))

(fn MakeRandomVectorwithThreshold
  (params (Min :type Float%20%28double-precision%29) (Max :type Float%20%28double-precision%29) (Threshold :type Float%20%28double-precision%29))
  (bind _output_get (LocalVariables|Setcurrent (Utilities|MakeRandomVector Min Max)))
  (while (< (Math|Vector|VectorLength _output_get) Threshold)
    (LocalVariables|Setcurrent (Utilities|MakeRandomVector Min Max))
    (Utilities|String|LogString "Value too low, rerandom"))
  (return (LocalVariables|Getcurrent)))

(fn CreateFaceWidgetArray
  (Variables|Default|SetFaceWidgetArray (Utilities|Array|MakeArray (Variables|Default|GetFaceWidgetTop) (Variables|Default|GetFaceWidgetLeft) (Variables|Default|GetFaceWidgetCenter) (Variables|Default|GetFaceWidgetRight) (Variables|Default|GetFaceWidgetEndRight) (Variables|Default|GetFaceWidgetBottom)))
  (return))

(fn SetDiceId
  (params (NewId :type Integer))
  (bind _faces (Variables|Default|GetFaces))
  (bind _output_get (Variables|Default|SetId NewId))
  (for (_ _array_index) _faces
    (Utilities|Struct|SetmembersinFace_Structure (Utilities|Array|Get(acopy) _faces _array_index) _output_get))
  (return))

(fn MouseIsOver
  (if (Variables|Default|GetIsMouseOver)
    _
    (else
      (Variables|Default|SetIsMouseOver true)
      (Default|CallDiceMouseEnter self)))
  (return))

(fn MouseNotOver
  (Default|CallDiceMouseExit self)
  (Variables|Default|SetIsMouseOver false))