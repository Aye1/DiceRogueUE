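; Base action Blueprint that evaluates a set of Faces, each carrying a map of element symbols to amounts.
; Execute and GetValueWithFaces are stubs, the latter returning zero, apparently meant for child actions to override.
; CountAllSymbols totals every amount across the faces, while SortSymbols merges the per-face maps into one map of summed amounts per symbol.
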(fn Execute
  (params (TargetComponent :type Targetable%20Component%20BP%20Object%20Reference) (Faces :type Array%20of%20Face%20Structure%20Structures)))

(fn CountAllSymbols
  (params (Faces :type Array%20of%20Face%20Structure%20Structures))
  (for _array_element Faces
    (bind _values (Utilities|Map|Values (.Elements (Utilities|Struct|BreakFace_Structure _array_element))))
    (for _array_element_2 _values
      (LocalVariables|SetSymbolsCount (+ _array_element_2 (LocalVariables|GetSymbolsCount)))))
  (return (LocalVariables|GetSymbolsCount)))

(fn GetValuewithFaces
  (params (Faces :type Array%20of%20Face%20Structure%20Structures))
  (return 0))

(fn SortSymbols
  (params (Faces :type Array%20of%20Face%20Structure%20Structures))
  (bind _symbolsmapping (LocalVariables|GetSymbolsMapping))
  (for _array_element Faces
    (bind _keys (Utilities|Map|Keys (.Elements (Utilities|Struct|BreakFace_Structure _array_element))))
    (for _array_element_2 _keys
      (if (.ReturnValue (Utilities|Map|Find (LocalVariables|GetSymbolsMapping) _array_element_2))
        (Utilities|Map|Add _symbolsmapping _array_element_2 (+ (.Value (Utilities|Map|Find (LocalVariables|GetSymbolsMapping) _array_element_2)) (.Value (Utilities|Map|Find (.Elements (Utilities|Struct|BreakFace_Structure _array_element)) _array_element_2))))
        (else
          (Utilities|Map|Add _symbolsmapping _array_element_2 (.Value (Utilities|Map|Find (.Elements (Utilities|Struct|BreakFace_Structure _array_element)) _array_element_2)))))))
  (return (LocalVariables|GetSymbolsMapping)))