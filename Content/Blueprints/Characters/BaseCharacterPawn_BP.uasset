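; BaseCharacterPawn_BP is the base pawn for combat characters that own dice, can be clicked to select, and can run a combat behavior tree.
; On BeginPlay it claims its dice, constructs actions from its classes, and announces initialization.
; It binds its health component to the target component and front and back health bars, and the target component to selection indicators.
; It also reports face-up dice, broadcasts plays, and destroys its dice on death.
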(event EventBeginPlay
  (Setup|AssignDiceOwnership)
  (Setup|BindObjects)
  (Setup|ConstructActions)
  (Selection|Unselect)
  (Default|CallOnInitialized self))

(event Collision|EventActorBeginOverlap
  (params (OtherActor :type Actor%20Object%20Reference)))

(event EventTick
  (params (DeltaSeconds :type Float%20%28single-precision%29)))

(event MouseInput|EventActorOnClicked
  (params (ButtonPressed :type Key%20Structure))
  (Default|CallOnSelected (Variables|Default|GetTargetComponent_BP))
  (Selection|Select))

(fn ConstructionScript)

(fn ConstructActions
  (for _array_element (Variables|Config|GetActionClasses)
    (bind _returnvalue (Game|ConstructObjectfromClass _array_element))
    (Utilities|Array|AddUnique (Variables|Default|GetActions) _returnvalue))
  (return))

(fn BindObjects
  (Variables|/Game/Blueprints/Characters/TargetableComponent_BP.TargetableComponent_BP_C|SetHealthComponent (Variables|Default|GetTargetComponent_BP) (Variables|Default|GetHealthComponent_BP))
  (Setup|BindHealthBar (Variables|Default|GetHealthBar))
  (Setup|BindHealthBar (Variables|Default|GetHealthBarBack))
  (Setup|BindSelectionIndicator (Variables|Default|GetSelectionIndicator))
  (Setup|BindSelectionIndicator (Variables|Default|GetSelectionIndicatorBack))
  (return))

(fn Select
  (Default|Select (Variables|Default|GetTargetComponent_BP))
  (return))

(fn Unselect
  (Default|Unselect (Variables|Default|GetTargetComponent_BP))
  (return))

(fn BindHealthBar
  (params (HealthBarWidgetComponent :type Widget%20Component%20Object%20Reference))
  (bind _ashealth_bar_widget_bp (Utilities|Casting|CastToHealthBarWidget_BP (UserInterface|GetUserWidgetObject HealthBarWidgetComponent)))
  (Default|SetHealthComponent _ashealth_bar_widget_bp (Variables|Default|GetHealthComponent_BP))
  (return))

(fn BindSelectionIndicator
  (params (SelectionWidgetComponent :type Widget%20Component%20Object%20Reference))
  (bind _asselection_indicator (Utilities|Casting|CastToSelectionIndicatorWidget_BP (UserInterface|GetUserWidgetObject SelectionWidgetComponent)))
  (Default|BindTargetComponent _asselection_indicator (Variables|Default|GetTargetComponent_BP))
  (return))

(fn AssignDiceOwnership
  (for _array_element (Variables|Config|GetDice)
    (Variables|/Game/Blueprints/Dice_BP.Dice_BP_C|SetCharacterOwner _array_element self))
  (return))

(fn GetCurrentFaces
  (for _array_element (Variables|Config|GetDice)
    (Utilities|Array|Add (LocalVariables|GetResult) (Variables|/Game/Blueprints/Dice_BP.Dice_BP_C|GetFaceUpInfo _array_element)))
  (return (LocalVariables|GetResult)))

(fn RunBehaviourTree
  (AI|RunBehaviorTree (AI|GetAIController self) "/Game/Blueprints/AI/BasicCombatBehaviourTree.BasicCombatBehaviourTree"))

(fn Play
  (params (SelectedPlay :type Play%20Evaluation%20BP%20Object%20Reference))
  (Default|CallOnPlays SelectedPlay)
  (Utilities|String|LogString "Play!")
  (return))

(fn Die
  (for _array_element (Variables|Config|GetDice)
    (Actor|DestroyActor _array_element))
  (Actor|DestroyActor))