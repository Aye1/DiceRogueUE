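; Base character pawn Blueprint that sets up its actions and health display when play begins.
; BeginPlay instantiates each entry in ActionClasses into the Actions list, binds components, then calls CallOnInitialized.
; Binding hands HealthComponentBP to the target component and to the front and back health bar widgets, so all share one health source.
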(event EventBeginPlay
  (CallFunction|ConstructActions)
  (CallFunction|BindObjects)
  (Default|CallOnInitialized))

(event Collision|EventActorBeginOverlap
  (params (OtherActor :type Actor%20Object%20Reference)))

(event EventTick
  (params (DeltaSeconds :type Float%20%28single-precision%29)))

(fn ConstructionScript)

(fn ConstructActions
  (for _array_element (Variables|Config|GetActionClasses)
    (bind _returnvalue (Game|ConstructObjectfromClass _array_element))
    (Utilities|Array|AddUnique (Variables|Default|GetActions) _returnvalue))
  (return))

(fn BindObjects
  (bind _healthcomponent_bp (Variables|Default|GetHealthComponent_BP))
  (Variables|/Game/Blueprints/Characters/TargetComponent_BP.TargetComponent_BP_C|SetHealthComponent (Variables|Default|GetTargetComponent_BP) _healthcomponent_bp)
  (bind _ashealth_bar_widget_bp (Utilities|Casting|CastToHealthBarWidget_BP (UserInterface|GetWidget (Variables|Default|GetHealthBar))))
  (Default|SetHealthComponent _ashealth_bar_widget_bp _healthcomponent_bp)
  (bind _ashealth_bar_widget_bp_2 (Utilities|Casting|CastToHealthBarWidget_BP (UserInterface|GetWidget (Variables|Default|GetHealthBarBack))))
  (Default|SetHealthComponent _ashealth_bar_widget_bp_2 _healthcomponent_bp)
  (return))