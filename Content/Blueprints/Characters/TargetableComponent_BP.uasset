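; Component that makes its owner targetable, tracking selection and passing damage and shield effects to a health component.
; Select and Unselect set the selection flag and broadcast OnSelect or OnUnselect with itself as the argument.
; DealDamage, which also logs the amount, and AddShield forward to HealthComponent through a shared validity-check macro, doing nothing when it is missing.
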(event EventBeginPlay)

(event EventTick
  (params (DeltaSeconds :type Float%20%28single-precision%29)))

(fn DealDamage
  (params (Damage :type Integer))
  (Utilities|String|LogString (Utilities|String|Append "Dealing damage: " (Utilities|String|ToString(Integer) Damage)))
  (bind _healthcomponent (Utilities|IsHealthComponentValid)
    (:True
      (Default|TakeDamage _healthcomponent Damage))
    (:False
      _))
  (return))

(fn AddShield
  (params (Shield :type Integer))
  (bind _healthcomponent (Utilities|IsHealthComponentValid)
    (:True
      (Default|AddShield _healthcomponent Shield))
    (:False
      _))
  (return))

(fn Select
  (Variables|Default|SetIsSelected true)
  (Default|CallOnSelect self))

(fn Unselect
  (Variables|Default|SetIsSelected false)
  (Default|CallOnUnselect self))