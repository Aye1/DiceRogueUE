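; Health component that tracks health, shield and death state, broadcasting events for health change, death and added shield.
; TakeDamage passes damage through BlockDamage, then lowers health or calls Die when the remainder reaches current health.
; BlockDamage drains shield without broadcasting, and zeroes it before subtracting, so a hit that breaks it deals full damage.
; Helpers add non-negative shield and return health as a fraction of maximum.
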(event EventBeginPlay)

(event EventTick
  (params (DeltaSeconds :type Float%20%28single-precision%29)))

(fn TakeDamage
  (params (Damage :type Integer))
  (bind _remainingdamage (CallFunction|BlockDamage Damage))
  (if (>= _remainingdamage (Variables|Default|GetCurrentHealth))
    (CallFunction|Die)
    (else
      (Variables|Default|SetCurrentHealth (- (Variables|Default|GetCurrentHealth) _remainingdamage))))
  (Default|CallOnHealthChanged)
  (return))

(fn Die
  (Variables|Default|SetCurrentHealth 0)
  (Variables|Default|SetIsDead true)
  (Default|CallOnDie self)
  (return))

(fn BlockDamage
  (params (Damage :type Integer))
  (if (>= Damage (Variables|Default|GetShield))
    (Variables|Default|SetShield 0)
    (return (- Damage (Variables|Default|GetShield)))
    (else
      (Variables|Default|SetShield (- (Variables|Default|GetShield) Damage))
      (return 0))))

(fn GetPercentHealth
  (return (Math|Float|SafeDivide (Math|Conversions|ToFloat(Integer) (Variables|Default|GetCurrentHealth)) (Math|Conversions|ToFloat(Integer) (Variables|Default|GetMaxHealth)))))

(fn AddShield
  (params (AddedShield :type Integer))
  (if (>= AddedShield 0)
    (Variables|Default|SetShield (+ AddedShield (Variables|Default|GetShield)))
    (Default|CallOnShieldChanged)
    (return)
    (else
      (Utilities|String|LogString "Ignoring negative shield"))))