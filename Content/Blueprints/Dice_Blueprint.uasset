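; Physics-driven six-sided die that rolls, reports its upward face and tints itself by Divinity (Fire, Water, Neutral).
; BeginPlay fills face and text-render arrays, then labels each side with its base value.
; RollDice applies a random off-centre impulse with a minimum strength and starts a minimum-roll timer.
; Tick detects rest after that timer, broadcasts the stop, then picks the face whose text scores highest on GetWorldAltitude, which reads world X.
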(event Collision|EventActorBeginOverlap
  (params (OtherActor :type Actor%20Object%20Reference)))

(event EventTick
  (params (DeltaSeconds :type Float%20%28single-precision%29))
  (Utilities|SetMaterialColorfromDivinity
    (:executeoutput
      (|SetIsInMotion)
      (Utilities|CheckIsRollFinished))))

(event EventBeginPlay
  (CallFunction|CreateTextRendersArray)
  (CallFunction|CreateFacesArray)
  (CallFunction|InitFaceValues))

(fn ConstructionScript)

(fn RollDice
  (Default|CallDiceStartedRolling self)
  (Utilities|String|LogString "Starting roll")
  (Variables|Default|SetIsRolling true)
  (Variables|Default|SetMinRollTimePassed false)
  (bind _result (CallFunction|MakeRandomVectorwithThreshold -2e+02 2e+02 5e+01))
  (Physics|AddImpulseatLocation (Variables|Default|GetCube) _result (Utilities|MakeRandomVector -5e+01 5e+01) "None")
  (CallFunction|StartRollTimer)
  (return))

(fn StartRollTimer
  (Utilities|Time|SetTimerbyFunctionName 0 "EndRollTimer" 1.0)
  (Utilities|String|LogString "Starting Roll Timer"))

(fn EndRollTimer
  (Variables|Default|SetMinRollTimePassed true)
  (Utilities|Time|ClearandInvalidateTimerbyHandle (Variables|Default|GetMinRollTimer))
  (Utilities|String|LogString "End Roll Timer"))

(fn InitFaceValues
  (for (_array_element _array_index) (Variables|Default|GetTextRendersArray)
    (Rendering|Components|TextRender|SetText _array_element (Utilities|Text|ToText(Integer) (Variables|/Game/Blueprints/DiceFaceComponent_Blueprint.DiceFaceComponent_Blueprint_C|GetBase%20Value (Utilities|Array|Get(acopy) (Variables|Default|GetFacesArray) _array_index))))
    (Utilities|String|LogString (Utilities|String|Append "Setting text to " (Utilities|String|ToString(Integer) (Variables|/Game/Blueprints/DiceFaceComponent_Blueprint.DiceFaceComponent_Blueprint_C|GetBase%20Value (Utilities|Array|Get(acopy) (Variables|Default|GetFacesArray) _array_index))) " for TextRender " (Utilities|GetObjectName _array_element)) false))
  (return))

(fn GetUpFacefromWorldLocation
  (LocalVariables|SetMaxAltitude -1e+05)
  (LocalVariables|SetMaxAltitudeFace -1)
  (for (_array_element _array_index) (Variables|Default|GetTextRendersArray)
    (if (> (Utilities|GetWorldAltitude _array_element) (LocalVariables|GetMaxAltitude))
      (LocalVariables|SetMaxAltitude (Utilities|GetWorldAltitude _array_element))
      (LocalVariables|SetMaxAltitudeFace (+ _array_index 1))))
  (Variables|Default|SetFaceUp (LocalVariables|GetMaxAltitudeFace))
  (return))

(fn CreateTextRendersArray
  (Utilities|Array|Clear (Variables|Default|GetTextRendersArray))
  (Utilities|AddTextRendertoArray (Variables|Default|GetTextRender1))
  (Utilities|AddTextRendertoArray (Variables|Default|GetTextRender2))
  (Utilities|AddTextRendertoArray (Variables|Default|GetTextRender3))
  (Utilities|AddTextRendertoArray (Variables|Default|GetTextRender4))
  (Utilities|AddTextRendertoArray (Variables|Default|GetTextRender5))
  (Utilities|AddTextRendertoArray (Variables|Default|GetTextRender6))
  (return))

(fn CreateFacesArray
  (Utilities|AddFacetoArray (Variables|Actor|GetDiceFace1)
    (:ExecuteOut
      (Utilities|AddFacetoArray (Variables|Default|GetDiceFace2)
        (:ExecuteOut
          (Utilities|AddFacetoArray (Variables|Default|GetDiceFace3)
            (:ExecuteOut
              (Utilities|AddFacetoArray (Variables|Default|GetDiceFace4)
                (:ExecuteOut
                  (Utilities|AddFacetoArray (Variables|Default|GetDiceFace5)
                    (:ExecuteOut
                      (Utilities|AddFacetoArray (Variables|Default|GetDiceFace6)
                        (:ExecuteOut
                          (return))))))))))))))

(fn MakeRandomVectorwithThreshold
  (params (Min :type Float%20%28double-precision%29) (Max :type Float%20%28double-precision%29) (Threshold :type Float%20%28double-precision%29))
  (bind _output_get (LocalVariables|Setcurrent (Utilities|MakeRandomVector Min Max)))
  (while (< (Math|Vector|VectorLength _output_get) Threshold)
    (LocalVariables|Setcurrent (Utilities|MakeRandomVector Min Max))
    (Utilities|String|LogString "Value too low, rerandom"))
  (return (LocalVariables|Getcurrent)))