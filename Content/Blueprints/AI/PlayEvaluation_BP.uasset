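; PlayEvaluation_BP is an AI data object representing a candidate play: dice faces assigned to actions, scored with a total value.
; An Actions map links each action to a FaceArray_BP wrapper, with CanAddFace checking the action's DiceMax limit.
; ComputeFinalValue sums each action's value for its assigned faces.
; Clone copies the assignments into a new evaluation without the computed Value, and Dump logs the contents for debugging.
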(fn ComputeFinalValue
  (bind _actions (Variables|Default|GetActions))
  (bind _keys (Utilities|Map|Keys _actions))
  (for _array_element _keys
    (if (not (Utilities|Array|IsEmpty (Variables|/Game/Blueprints/AI/FaceArray_BP.FaceArray_BP_C|GetFaces (.Value (Utilities|Map|Find _actions _array_element)))))
      (bind _value (Default|GetValuewithFaces _array_element (Variables|/Game/Blueprints/AI/FaceArray_BP.FaceArray_BP_C|GetFaces (.Value (Utilities|Map|Find _actions _array_element)))))
      (LocalVariables|SetCurrentValue (+ _value (LocalVariables|GetCurrentValue)))))
  (bind _output_get (Variables|Default|SetValue (LocalVariables|GetCurrentValue)))
  (return _output_get))

(fn AddFacetoAction
  (params (Action :type Action%20BP%20Object%20Reference) (Face :type Face%20Structure%20Structure))
  (bind _actions (Variables|Default|GetActions))
  (bind (_value _returnvalue) (Utilities|Map|Find _actions Action))
  (if _returnvalue
    (Utilities|Array|Add (Variables|/Game/Blueprints/AI/FaceArray_BP.FaceArray_BP_C|GetFaces _value) Face)
    (return)
    (else
      (bind _returnvalue_2 (Game|ConstructObjectfromClass "/Game/Blueprints/AI/FaceArray_BP.FaceArray_BP_C"))
      (Default|AddFace _returnvalue_2 Face)
      (Utilities|Map|Add _actions Action _returnvalue_2)
      (return))))

(fn CanAddFace
  (params (Action :type Action%20BP%20Object%20Reference))
  (bind _actions (Variables|Default|GetActions))
  (bind (_value _returnvalue) (Utilities|Map|Find _actions Action))
  (if _returnvalue
    (return (< (Utilities|Array|Length (Variables|/Game/Blueprints/AI/FaceArray_BP.FaceArray_BP_C|GetFaces _value)) (.DiceMax (Utilities|Struct|BreakAction_Structure (Variables|/Game/Blueprints/Actions/Action_BP.Action_BP_C|GetActionInfo Action)))))
    (else
      (return true))))

(fn Dump
  (params (PrintToLog :type Boolean))
  (bind _actions (Variables|Default|GetActions))
  (Utilities|String|LogString "==Dumping PlayEvaluation==" PrintToLog)
  (bind _keys (Utilities|Map|Keys _actions))
  (for _array_element _keys
    (Utilities|String|LogString (Utilities|String|Append (Utilities|GetObjectName _array_element) " - " (Utilities|String|ToString(Integer) (Utilities|Array|Length (Variables|/Game/Blueprints/AI/FaceArray_BP.FaceArray_BP_C|GetFaces (.Value (Utilities|Map|Find _actions _array_element))))) " element(s)") PrintToLog))
  (Utilities|String|LogString (Utilities|String|Append "Total value - " (Utilities|String|ToString(Integer) (Variables|Default|GetValue))) PrintToLog)
  (Utilities|String|LogString "==========================" PrintToLog)
  (return))

(fn Clone
  (bind _actions (Variables|Default|GetActions))
  (bind _returnvalue (Game|ConstructObjectfromClass "PlayEvaluation_BP_C"))
  (bind _keys (Utilities|Map|Keys _actions))
  (for _array_element _keys
    (for _array_element_2 (Variables|/Game/Blueprints/AI/FaceArray_BP.FaceArray_BP_C|GetFaces (.Value (Utilities|Map|Find _actions _array_element)))
      (CallFunction|AddFacetoAction _returnvalue _array_element _array_element_2)))
  (return _returnvalue))