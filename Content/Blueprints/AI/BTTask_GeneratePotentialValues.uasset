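; Behavior tree task that enumerates every valid way the AI pawn can assign its current Faces to its Actions.
; Compute recursively takes the last Face and branches on a cloned PlayEvaluation for each Action that passes CanAddFace, with a depth cap as a safety stop.
; Completed plays collect in an AllPlayEvaluations object, which computes their values and is stored in the PotentialPlays Blackboard key.
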(event EventReceiveExecuteAI
  (params (OwnerController :type AI%20Controller%20Object%20Reference) (ControlledPawn :type Pawn%20Object%20Reference))
  (bind _allplayevaluations (Variables|Default|GetAllPlayEvaluations))
  (bind _asbase_character_pawn (Utilities|Casting|CastToBaseCharacterPawn ControlledPawn)
    (:then
      (CallFunction|Init)
      (bind _faces (Default|GetCurrentFaces _asbase_character_pawn))
      (bind _output_get (Variables|Default|SetFaces _faces))
      (bind _output_get_2 (Variables|Default|SetActions (Variables|/Game/Blueprints/Characters/BaseCharacterPawn.BaseCharacterPawn_C|GetActions _asbase_character_pawn)))
      (bind _returnvalue (Game|ConstructObjectfromClass "/Game/Blueprints/AI/PlayEvaluation_BP.PlayEvaluation_BP_C"))
      (CallFunction|Compute _returnvalue _output_get _output_get_2 5)
      (Default|ComputeValues _allplayevaluations)
      (Class|BTFunctionLibrary|SetBlackboardValueasObject (Variables|Default|GetPotentialPlays) _allplayevaluations)
      (AI|BehaviorTree|FinishExecute true))
    (:CastFailed
      (Utilities|String|LogString "Cast failed - see BTTask_GeneratePotentialValues")
      (AI|BehaviorTree|FinishExecute false))))

(fn Compute
  (params (Current :type Play%20Evaluation%20BP%20Object%20Reference) (AvailableFaces :type Array%20of%20Face%20Structure%20Structures) (AvailableActions :type Array%20of%20Action%20BP%20Object%20References) (SafetyMaxLevel :type Integer))
  (if (> SafetyMaxLevel 0)
    (if (Utilities|Array|IsEmpty AvailableFaces)
      ;[0.15 0.15 0.15 0.5] End recursion - no Face remaining
      (Default|Add (Variables|Default|GetAllPlayEvaluations) Current)
      (Utilities|String|LogString "Recursion ended properly" false)
      (Default|Dump Current false)
      (return)
      (else
        (bind (_element _remaining) (CallFunction|ExtractLastElementfromArray AvailableFaces))
        (for _array_element AvailableActions
          (if (Default|CanAddFace Current _array_element)
            (bind _clone (Default|Clone Current))
            (Default|AddFacetoAction _clone _array_element _element)
            (CallFunction|Compute _clone _remaining AvailableActions (- SafetyMaxLevel 1))))
        (return)))
    (else
      (Utilities|String|LogString "Hit safetly max level! Exiting")
      (return))))

(fn ExtractLastElementfromArray
  (params (Faces :type Array%20of%20Face%20Structure%20Structures))
  (bind _returnvalue (Utilities|Array|Length Faces))
  (bind _returnvalue_2 (- _returnvalue 1))
  (for (_array_element _array_index) Faces
    (if (!= _array_index _returnvalue_2)
      (Utilities|Array|Add (LocalVariables|GetNewArray) _array_element) ; Populate new array with all elements except last
    ))
  (return (Utilities|Array|Get(acopy) Faces _returnvalue_2) (LocalVariables|GetNewArray)))

(fn Init
  (bind _returnvalue (Game|ConstructObjectfromClass "/Game/Blueprints/AI/AllPlayEvaluation_BP.AllPlayEvaluation_BP_C"))
  (Variables|Default|SetAllPlayEvaluations _returnvalue)
  (return))