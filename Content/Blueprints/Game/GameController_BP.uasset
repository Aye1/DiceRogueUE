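; Central controller for dice-based, turn-based combat between Player and Enemies teams.
; It creates the main HUD, registers characters as targets, and relays their dice, actions and plays to the UI.
; It tracks rolling dice to detect when all stop, and sends StateTree events to end phases.
; Enemy actions come from behaviour trees, and character deaths trigger victory or defeat checks.
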(event Custom|OnDiceStoppedRolling
  (params (Dice :type Dice%20BP%20Object%20Reference%20%28by%20ref%29))
  (Utilities|Map|Add (Variables|State|GetRollingDice) Dice false)
  (Dice|CheckIsRolling))

(event Custom|OnDiceStartedRolling
  (params (Dice :type Dice%20BP%20Object%20Reference%20%28by%20ref%29))
  (Utilities|Map|Add (Variables|State|GetRollingDice) Dice true)
  (Variables|State|SetRollInProgress true))

(event EventBeginPlay
  (UISetup|CreateUI)
  (Bindings|BindEvents)
  (CallFunction|RegisterTargets)
  (Bindings|BindDebugActor))

(event Collision|EventActorBeginOverlap
  (params (OtherActor :type Actor%20Object%20Reference)))

(event EventTick
  (params (DeltaSeconds :type Float%20%28single-precision%29)))

(event Custom|OnRollButtonPressed
  (Dice|RollDiceforTeam "NewEnumerator0"))

(fn ConstructionScript)

(fn CreateUI
  (bind _returnvalue (UserInterface|CreateWidget "/Game/Blueprints/UI/MainHUDWidget_BP.MainHUDWidget_BP_C"))
  (bind _output_get (Variables|Default|SetHUDReference _returnvalue))
  (UserInterface|Viewport|AddtoViewport _output_get 0)
  (Default|SetGameController _output_get self)
  (Default|SetSelectionController _output_get (Variables|WorldBindings|GetSelectionControllerRef))
  (return))

(fn BindEvents
  (for _array_element (Variables|WorldBindings|GetCharacters)
    (Bindings|BindCharacterEvents _array_element))
  (return))

(fn BindDiceEvents
  (params (Dice :type Dice%20BP%20Object%20Reference))
  (EventDispatchers|BindEventtoDiceStartedRolling Dice (EventDispatchers|CreateEvent :!event Custom|OnDiceStartedRolling))
  (EventDispatchers|BindEventtoDiceStoppedRolling Dice (EventDispatchers|CreateEvent :!event Custom|OnDiceStoppedRolling))
  (return))

(fn CheckIsRolling
  (LocalVariables|SetIsRolling false)
  (bind _values (Utilities|Map|Values (Variables|State|GetRollingDice)))
  (bind _array_element (Utilities|Array|ForEachLoopwithBreak _values :!label _label)
    (:LoopBody
      (if _array_element
        (LocalVariables|SetIsRolling true)
        (goto _label Break)))
    (:Completed
      (if (and (Variables|State|GetRollInProgress) (not (LocalVariables|GetIsRolling)))
        (Variables|State|SetRollInProgress false)
        (Default|CallOnAllDiceStoppedRolling)
        (if (Utilities|Enum|Equal(Enum) (Variables|Default|GetCurrentRollTeam) "NewEnumerator1")
          (StateTree|SendStateEvent "(TagName=\"StateTree.Combat.EnemiesRollDice.End\")")))
      (return))))

(fn RollDice
  (params (DiceArray :type Array%20of%20Dice%20BP%20Object%20References))
  (Variables|State|SetRollInProgress true)
  (Default|CallOnDiceStartRolling)
  (for _array_element DiceArray
    (Default|RollDice _array_element))
  (return))

(fn SendDicetoUI
  (params (Character :type Base%20Character%20Pawn%20BP%20Object%20Reference))
  (Default|AddDiceArray (Variables|Default|GetHUDReference) (Variables|/Game/Blueprints/Characters/BaseCharacterPawn_BP.BaseCharacterPawn_BP_C|GetDice Character)))

(fn SendActionstoUI
  (params (Character :type Base%20Character%20Pawn%20BP%20Object%20Reference))
  (Default|AddActions (Variables|Default|GetHUDReference) Character)
  (return))

(fn InitCombat
  (Utilities|String|LogString "Init game - does nothing at the moment"))

(fn StartPlayerPlanPhase
  (Default|CallOnPlayerPlanPhaseStart)
  (return))

(fn OnCharacterInitialized
  (params (Character :type Base%20Character%20Pawn%20BP%20Object%20Reference))
  (Dice|SetDiceId Character)
  (UISetup|SendDicetoUI Character)
  (UISetup|SendActionstoUI Character))

(fn RegisterTargets
  (bind _selectioncontrollerref (Variables|WorldBindings|GetSelectionControllerRef))
  (for _array_element (Variables|WorldBindings|GetCharacters)
    (Default|RegisterTargetable _selectioncontrollerref (Variables|/Game/Blueprints/Characters/BaseCharacterPawn_BP.BaseCharacterPawn_BP_C|GetTargetComponent_BP _array_element) (Variables|/Game/Blueprints/Characters/BaseCharacterPawn_BP.BaseCharacterPawn_BP_C|GetTeam _array_element)))
  (Default|SelectRandomTarget _selectioncontrollerref)
  (return))

(fn StartEnemiesPlanPhase
  (Default|CallOnEnemiesPlanPhaseStart)
  (Dice|RollDiceforTeam "NewEnumerator1")
  (return))

(fn GetDiceforTeam
  (params (Team :type TeamEnum%20Enum :default "NewEnumerator0"))
  (for _array_element (Variables|WorldBindings|GetCharacters)
    (if (Utilities|Enum|Equal(Enum) Team (Variables|/Game/Blueprints/Characters/BaseCharacterPawn_BP.BaseCharacterPawn_BP_C|GetTeam _array_element))
      (Utilities|Array|AppendArray (LocalVariables|GetDiceArray) (Variables|/Game/Blueprints/Characters/BaseCharacterPawn_BP.BaseCharacterPawn_BP_C|GetDice _array_element))))
  (return (LocalVariables|GetDiceArray)))

(fn RollDiceforTeam
  (params (Team :type TeamEnum%20Enum :default "NewEnumerator0"))
  (bind _output_get (Variables|Default|SetCurrentRollTeam Team))
  (bind _dice (Dice|GetDiceforTeam _output_get))
  (Dice|RollDice _dice)
  (return))

(fn BindCharacterEvents
  (params (Character :type Base%20Character%20Pawn%20BP%20Object%20Reference))
  (for _array_element (Variables|/Game/Blueprints/Characters/BaseCharacterPawn_BP.BaseCharacterPawn_BP_C|GetDice Character)
    (Bindings|BindDiceEvents _array_element))
  (EventDispatchers|BindEventtoOnInitialized Character (EventDispatchers|CreateEvent :!event OnCharacterInitialized))
  (EventDispatchers|BindEventtoOnPlays Character (EventDispatchers|CreateEvent :!event OnCharacterPlays))
  (EventDispatchers|BindEventtoOnDie (Variables|/Game/Blueprints/Characters/BaseCharacterPawn_BP.BaseCharacterPawn_BP_C|GetHealthComponent_BP Character) (EventDispatchers|CreateEvent :!event OnCharacterDies))
  (return))

(fn DecideEnemiesActions
  (for _array_element (Variables|WorldBindings|GetCharacters)
    (if (Utilities|Enum|Equal(Enum) (Variables|/Game/Blueprints/Characters/BaseCharacterPawn_BP.BaseCharacterPawn_BP_C|GetTeam _array_element) "NewEnumerator1")
      (Default|RunBehaviourTree _array_element))))

(fn OnCharacterPlays
  (params (Play :type Play%20Evaluation%20BP%20Object%20Reference))
  (Default|SetupPlay (Variables|Default|GetHUDReference) Play)
  (Utilities|String|LogString "Setup play"))

(fn SetDiceId
  (params (Character :type Base%20Character%20Pawn%20BP%20Object%20Reference))
  (for _array_element (Variables|/Game/Blueprints/Characters/BaseCharacterPawn_BP.BaseCharacterPawn_BP_C|GetDice Character)
    (Default|SetDiceId _array_element (Variables|Default|GetLatestDiceId))
    (Variables|Default|SetLatestDiceId (+ (Variables|Default|GetLatestDiceId) 1))))

(fn ExecuteActions
  (params (Team :type TeamEnum%20Enum :default "NewEnumerator0"))
  (Default|ExecuteActions (Variables|Default|GetHUDReference) Team)
  (return))

(fn EndPlayerPlanPhase
  (StateTree|SendStateEvent "(TagName=\"StateTree.Combat.PlayerPlan.End\")")
  (return))

(fn OnCharacterDies
  (params (HealthComponent :type Health%20Component%20BP%20Object%20Reference))
  (bind _asbase_character_pawn_bp (Utilities|Casting|CastToBaseCharacterPawn_BP (Components|GetOwner HealthComponent))
    (:then
      (Utilities|Array|RemoveItem (Variables|WorldBindings|GetCharacters) _asbase_character_pawn_bp)
      (Default|RemoveCharacter (Variables|Default|GetHUDReference) _asbase_character_pawn_bp)
      (Default|UnregisterTargetable (Variables|WorldBindings|GetSelectionControllerRef) (Variables|/Game/Blueprints/Characters/BaseCharacterPawn_BP.BaseCharacterPawn_BP_C|GetTargetComponent_BP _asbase_character_pawn_bp))
      (Default|Die _asbase_character_pawn_bp)
      (CallFunction|CheckCombatEnd))
    (:CastFailed
      (Utilities|String|LogString "Failed to cast - see GameController_BP - OnCharacterDies")))
  (return))

(fn CheckCombatEnd
  (for _array_element (Variables|WorldBindings|GetCharacters)
    (switch Utilities|FlowControl|Switch|SwitchonTeamEnum (Variables|/Game/Blueprints/Characters/BaseCharacterPawn_BP.BaseCharacterPawn_BP_C|GetTeam _array_element)
      (:NewEnumerator0
        (Math|Integer|IncrementInt (LocalVariables|GetPlayerCount)))
      (:NewEnumerator1
        (Math|Integer|IncrementInt (LocalVariables|GetEnemiesCount)))))
  (if (== (LocalVariables|GetPlayerCount) 0)
    (CallFunction|EndCombat "NewEnumerator1")
    (Default|CallOnDefeat)
    (elif (== (LocalVariables|GetEnemiesCount) 0)
      (CallFunction|EndCombat "NewEnumerator0")
      (Default|CallOnVictory)
      (else
        (return))))
  (return))

(fn EndCombat
  (params (Winner :type TeamEnum%20Enum :default "NewEnumerator0")))

(fn SendStateEvent
  (params (Tag :type Gameplay%20Tag%20Structure))
  (Gameplay|StateTree|SendStateTreeEvent (Variables|Default|GetStateTree) (Utilities|Struct|MakeStateTreeEvent Tag) :!class /Script/GameplayStateTreeModule.StateTreeComponent)
  (return))

(fn BindDebugActor
  (Default|SetDebugActor (Variables|Default|GetHUDReference) (Variables|WorldBindings|GetDebugActor))
  (return))

(fn SetTargetforAction
  (params (ActionInfo :type Action%20Structure%20Structure) (Team :type TeamEnum%20Enum :default "NewEnumerator0"))
  (Default|SelectTargetforActionbyTeam (Variables|WorldBindings|GetSelectionControllerRef) ActionInfo Team))