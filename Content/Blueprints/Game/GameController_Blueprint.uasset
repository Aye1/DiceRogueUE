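; Game controller for a dice-based game that manages the player's dice rolls and action planning, with combat logic still stubbed.
; On BeginPlay it creates the main HUD, binds dice events, and passes the player's dice and actions to the HUD.
; A per-die rolling map detects when all dice stop and fires an event.
; ApplyActions reads each action's faces from the HUD, but applying, validating and combat setup are mostly logging placeholders.
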(event Custom|OnDiceStoppedRolling
  (params (Dice :type Dice%20Blueprint%20Object%20Reference%20%28by%20ref%29))
  (Utilities|Map|Add (Variables|Default|GetPlayerRollingDice) Dice false)
  (CallFunction|CheckIsRolling))

(event Custom|OnDiceStartedRolling
  (params (Dice :type Dice%20Blueprint%20Object%20Reference%20%28by%20ref%29))
  (Utilities|Map|Add (Variables|Default|GetPlayerRollingDice) Dice true)
  (Variables|Default|SetPlayerRollInProgress true))

(event EventBeginPlay
  (CallFunction|CreateUI)
  (CallFunction|BindEvents)
  (CallFunction|SendDicetoUI)
  (CallFunction|SendActionstoUI))

(event Collision|EventActorBeginOverlap
  (params (OtherActor :type Actor%20Object%20Reference)))

(event EventTick
  (params (DeltaSeconds :type Float%20%28single-precision%29)))

(event Custom|OnRollButtonPressed
  (Variables|Default|SetPlayerRollInProgress true)
  (CallFunction|RollDice (Variables|Default|GetPlayerDice)))

(event Custom|OnValidateButtonPressed
  (Utilities|String|LogString "Validate")
  (Variables|Default|SetPlayerPlanPhaseTMP false))

(fn ConstructionScript)

(fn CreateUI
  (bind _returnvalue (UserInterface|CreateWidget "/Game/Blueprints/UI/MainHUDWidget_Blueprint.MainHUDWidget_Blueprint_C"))
  (bind _output_get (Variables|Default|SetHUDReference _returnvalue))
  (UserInterface|Viewport|AddtoViewport _output_get 0)
  (Default|SetGameController _output_get self)
  (return))

(fn BindEvents
  (for _array_element (Variables|Default|GetPlayerDice)
    (CallFunction|BindDiceEvents _array_element))
  (return))

(fn BindDiceEvents
  (params (Dice :type Dice%20Blueprint%20Object%20Reference))
  (EventDispatchers|BindEventtoDiceStartedRolling Dice (EventDispatchers|CreateEvent :!event Custom|OnDiceStartedRolling))
  (EventDispatchers|BindEventtoDiceStoppedRolling Dice (EventDispatchers|CreateEvent :!event Custom|OnDiceStoppedRolling))
  (return))

(fn CheckIsRolling
  (LocalVariables|SetIsRolling false)
  (bind _values (Utilities|Map|Values (Variables|Default|GetPlayerRollingDice)))
  (bind _array_element (Utilities|Array|ForEachLoopwithBreak _values :!label _label)
    (:LoopBody
      (if _array_element
        (LocalVariables|SetIsRolling true)
        (goto _label Break)))
    (:Completed
      (if (and (Variables|Default|GetPlayerRollInProgress) (not (LocalVariables|GetIsRolling)))
        (Variables|Default|SetPlayerRollInProgress false)
        (Default|CallOnAllDiceStoppedRolling))
      (return))))

(fn RollDice
  (params (DiceArray :type Array%20of%20Dice%20Blueprint%20Object%20References))
  (Default|CallOnDiceStartRolling)
  (for _array_element DiceArray
    (Default|RollDice _array_element))
  (return))

(fn SendDicetoUI
  (Default|AddDiceArray (Variables|Default|GetHUDReference) (Variables|Default|GetPlayerDice))
  (return))

(fn SendActionstoUI
  (Default|AddActions (Variables|Default|GetHUDReference) (Variables|Default|GetPlayerActions))
  (return))

(fn InitCombat
  (Utilities|String|LogString "Init game - does nothing at the moment"))

(fn StartPlayerPlanPhase
  (Variables|Default|SetPlayerPlanPhaseTMP true)
  (Default|CallOnPlayerPlanPhaseStart)
  (return))

(fn ApplyActions
  (bind _hudreference (Variables|Default|GetHUDReference))
  (for _array_element (Variables|Default|GetPlayerActions)
    (bind _faces (Default|GetFacesforAction _hudreference _array_element))
    (CallFunction|ApplyAction _array_element _faces))
  (Default|ResetActions _hudreference)
  (return))

(fn ApplyAction
  (params (Action :type Action%20Structure%20Structure) (Faces :type Array%20of%20Face%20Structure%20Structures))
  (Utilities|String|LogString (Utilities|String|Append "Doing action " (.Name (Utilities|Struct|BreakAction_Structure Action)) " with " (Utilities|String|ToString(Integer) (Utilities|Array|Length Faces)) " dice")))