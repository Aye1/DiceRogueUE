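; Selection controller that tracks targetable characters by team and manages which one is selected.
; Registering adds a targetable to a team map and binds its select/unselect events; selecting one stores it and unselects all others.
; It can select a random target, or the first on the team suited to an action: opponents for Attack, the acting team for Block or Heal.
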(event EventBeginPlay)

(event Collision|EventActorBeginOverlap
  (params (OtherActor :type Actor%20Object%20Reference)))

(event EventTick
  (params (DeltaSeconds :type Float%20%28single-precision%29)))

(fn ConstructionScript)

(fn RegisterTargetable
  (params (Targetable :type Targetable%20Component%20BP%20Object%20Reference) (Team :type TeamEnum%20Enum :default "NewEnumerator0"))
  (Utilities|Map|Add (Variables|Default|GetTargetableMap) Targetable Team)
  (CallFunction|BindTargetEvents Targetable))

(fn UnregisterTargetable
  (params (TargetComponent :type Targetable%20Component%20BP%20Object%20Reference))
  (Utilities|Map|Remove (Variables|Default|GetTargetableMap) TargetComponent)
  (return))

(fn OnCharacterSelected
  (params (TargetComponent :type Targetable%20Component%20BP%20Object%20Reference))
  (Variables|Default|SetSelectedCharacter TargetComponent)
  (bind _keys (Utilities|Map|Keys (Variables|Default|GetTargetableMap)))
  (for _array_element _keys
    (if (!= _array_element TargetComponent)
      (Default|Unselect _array_element)))
  (return))

(fn BindTargetEvents
  (params (Targetable :type Targetable%20Component%20BP%20Object%20Reference))
  (EventDispatchers|BindEventtoOnSelect Targetable (EventDispatchers|CreateEvent :!event OnCharacterSelected))
  (EventDispatchers|BindEventtoOnUnselect Targetable (EventDispatchers|CreateEvent :!event OnCharacterUnselected))
  (return))

(fn OnCharacterUnselected
  (params (Targetable :type Targetable%20Component%20BP%20Object%20Reference)))

(fn SelectRandomTarget
  (bind _keys (Utilities|Map|Keys (Variables|Default|GetTargetableMap)))
  (Default|Select (.OutItem (Utilities|Array|Random _keys))))

(fn SelectFirstTargetforActionbyTeam
  (params (ActionInfo :type Action%20Structure%20Structure) (Team :type TeamEnum%20Enum :default "NewEnumerator0"))
  (bind _category (Utilities|Struct|BreakAction_Structure ActionInfo))
  (bind _targetablemap (Variables|Default|GetTargetableMap))
  (switch Utilities|FlowControl|Switch|SwitchonTeamEnum Team
    (:NewEnumerator0
      (switch Utilities|FlowControl|Switch|SwitchonActionCategoryEnum _category
        (:NewEnumerator0
          (LocalVariables|SetTargetTeam "NewEnumerator1" :!label _label))
        (:NewEnumerator1
          (LocalVariables|SetTargetTeam "NewEnumerator0" :!label _label_2))
        (:NewEnumerator2
          (goto _label_2))))
    (:NewEnumerator1
      (switch Utilities|FlowControl|Switch|SwitchonActionCategoryEnum _category
        (:NewEnumerator0
          (goto _label_2))
        (:NewEnumerator1
          (goto _label))
        (:NewEnumerator2
          (goto _label)))))
  (bind _keys (Utilities|Map|Keys _targetablemap))
  (bind _array_element (Utilities|Array|ForEachLoopwithBreak _keys :!label _label_3)
    (:LoopBody
      (if (Utilities|Enum|Equal(Enum) (LocalVariables|GetTargetTeam) (.Value (Utilities|Map|Find _targetablemap _array_element)))
        (Default|Select _array_element)
        (goto _label_3 Break)))
    (:Completed
      (return))))